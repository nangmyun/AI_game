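; BP_LearningTrainerB is a Learning Agents trainer that defines rewards and episode resets for BP_AICharacterB agents.
; Each agent earns a positive reward when its rotation trace hits red and a smaller penalty when it dies.
; Completion always reports Running, so episodes never end from this logic.
; Resets send each agent back to its point, and agent 0 also resets the scoreboard.
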(fn `GatherAgentCompletion`
  (params (AgentId :type Integer))
  (returns (OutCompletion :type "ELearningAgentsCompletion Enum"))
  (return "Running"))

(fn `GatherAgentReward`
  (params (AgentId :type Integer))
  (returns (OutReward :type "Float (single-precision)"))
  (set `self.RewardActor` (`self.GetAgent` AgentId "/Game/ThirdPerson/Blueprints/BP_AICharacterB.BP_AICharacterB_C"))
  (bind (_hitblue _hitred) (`/Game/ThirdPerson/Blueprints/BP_AICharacterB.TraceRotation` (`self.RewardActor`)))
  (return (+ (`LearningAgentsRewards.MakeRewardOnCondition` _hitred 10.0 "ConditionReward" false null) (`LearningAgentsRewards.MakeRewardOnCondition` (`/Game/ThirdPerson/Blueprints/BP_AICharacterB.Death` (`self.RewardActor`)) -2.5 "ConditionReward" false null))))

(fn `ResetAgentEpisode`
  (params (AgentId :type Integer))
  (bind _returnvalue (`self.GetAgent` AgentId "/Game/ThirdPerson/Blueprints/BP_AICharacterB.BP_AICharacterB_C"))
  (`/Game/ThirdPerson/Blueprints/BP_AICharacterB.ResetToPoint` _returnvalue)
  (if (== AgentId 0)
    (`/Game/ThirdPerson/Blueprints/BP_AICharacterB.ResetScoreBoard` _returnvalue)))